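; BP_Projectile is a projectile that delivers damage through the Gameplay Ability System.
; On hit, if the struck actor has an Ability System Component, it sets the effect context origin to the impact point, applies the stored damage spec to that component, then destroys itself.
; A separate event tints the mesh through its Base Color material parameter.
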(event EventBeginPlay
  (|CallParentFunction))

(event EventSetMeshColor
  (params (MeshColor :type Linear%20Color%20Structure%20%28by%20ref%29))
  (Rendering|Material|SetVectorParameterValueonMaterials (Variables|Default|GetMesh) "Base Color" (Math|Conversions|ToVector(LinearColor) MeshColor)))

(event EventOnProjectileHit
  (params (Hit :type Hit%20Result%20Structure%20%28by%20ref%29))
  (bind (_bblockinghit _binitialoverlap _time _distance _location _impactpoint _normal _impactnormal _physmat _hitactor) (Collision|BreakHitResult Hit))
  (bind _damagespechandle (Variables|Default|GetDamageSpecHandle))
  (bind _returnvalue (Ability|GetAbilitySystemComponent _hitactor))
  (Utilities|IsValid _returnvalue
    (:Is%20Valid
      (bind _returnvalue_2 (Class|AbilitySystemBlueprintLibrary|GetEffectContext _damagespechandle))
      (Class|AbilitySystemBlueprintLibrary|EffectContextSetOrigin _returnvalue_2 _impactpoint)
      (GameplayEffects|ApplyGameplayEffectSpecToSelf _returnvalue _damagespechandle)
      (Actor|DestroyActor))))

(fn ConstructionScript)